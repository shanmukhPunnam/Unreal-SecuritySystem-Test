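; Test security camera actor that recolors its spotlight according to where the player stands relative to its facing.
; Each Tick it measures distance to the player and derives a 0–360 horizontal angle from the forward vector using cross and dot products with Atan2.
; Out of range or behind shows green, a narrow front cone shows red, and the side arcs show amber.
; It only checks range and angle, with no line-of-sight test.
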(event EventTick
  (params (DeltaSeconds :type Float%20%28single-precision%29))
  (bind _returnvalue (Game|GetPlayerCharacter 0))
  (bind _returnvalue_2 (Transformation|GetActorLocation))
  (bind _returnvalue_3 (Transformation|GetActorForwardVector))
  (bind _returnvalue_4 (Transformation|GetActorLocation _returnvalue))
  (bind _returnvalue_5 (Math|Conversions|ToVector2D(Vector) _returnvalue_3))
  (bind _returnvalue_6 (- _returnvalue_4 _returnvalue_2))
  (bind _returnvalue_7 (Math|Conversions|ToVector2D(Vector) _returnvalue_6))
  (bind _returnvalue_8 (Math|Vector|CrossProduct _returnvalue_6 _returnvalue_3))
  (bind _returnvalue_9 (Math|Vector2D|DotProduct(2D) _returnvalue_7 _returnvalue_5))
  (bind _z (Math|Vector|BreakVector _returnvalue_8))
  (bind _returnvalue_10 (Math|Trig|Atan2(Radians) _z _returnvalue_9))
  (bind _returnvalue_11 (Math|Trig|RadiansToDegrees _returnvalue_10))
  (Variables|Default|SetDistance (Math|Vector|VectorLength (- _returnvalue_4 _returnvalue_2)))
  (bind _output_get (Variables|Default|Setcurrent%20Angle (Math|Float|SelectFloat (+ 3.6e+02 _returnvalue_11) _returnvalue_11 (< _returnvalue_11 0.0))))
  (if (>= (Variables|Default|GetDistance) 2e+03)
    (Variables|Default|SetLight%20Color (Math|Conversions|ToColor(LinearColor) (Math|Color|SelectColor :A "(R=0.013723,G=1.000000,B=0.000000,A=1.000000)" :bPickA true)))
    (elif (or (<= _output_get 3e+01) (>= _output_get 3.3e+02))
      (Variables|Default|SetLight%20Color (Math|Conversions|ToColor(LinearColor) (Math|Color|SelectColor :A "(R=1.000000,G=0.000000,B=0.033848,A=1.000000)" :bPickA true)))
      (elif (or (and (>= _output_get 3e+01) (<= _output_get 1.5e+02)) (and (>= _output_get 2.1e+02) (<= _output_get 3.3e+02)))
        (Variables|Default|SetLight%20Color (Math|Conversions|ToColor(LinearColor) (Math|Color|SelectColor :A "(R=1.000000,G=0.730212,B=0.000000,A=1.000000)" :bPickA true)))
        (else
          (Variables|Default|SetLight%20Color (Math|Conversions|ToColor(LinearColor) (Math|Color|SelectColor :A "(R=0.000000,G=1.000000,B=0.153402,A=1.000000)" :bPickA true)))))))
  (Rendering|Components|Light|SetLightColor (Variables|Default|GetSpotLight) (Math|Conversions|ToLinearColor(Color) (Variables|Default|GetLight%20Color)) true))

(fn ConstructionScript)