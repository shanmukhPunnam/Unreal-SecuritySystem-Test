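; BP_Keypad is a test keypad actor that opens the keypad UI when its Cube component registers a hit.
; The hit adds new keypad and gameplay widgets, shows the mouse cursor and sets CanShowCamera on the first BP_SecurityCamera found.
; It has no check on the hitting actor or for existing widgets.
; Escape toggles cursor visibility through a FlipFlop, and a leftover node chain never runs.
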(event OnComponentHit(Cube)
  (params (HitComponent :type Primitive%20Component%20Object%20Reference) (OtherActor :type Actor%20Object%20Reference) (OtherComp :type Primitive%20Component%20Object%20Reference) (NormalImpulse :type Vector :default "0, 0, 0") (Hit :type Hit%20Result%20Structure%20%28by%20ref%29))
  (bind _returnvalue (UserInterface|CreateWidget "/Game/Test/WBP_KeypadUI.WBP_KeypadUI_C"))
  (UserInterface|Viewport|AddtoViewport _returnvalue 0)
  (Variables|/Script/Engine.PlayerController|SetbShowMouseCursor (Game|GetPlayerController 0) true)
  (bind _outactors (Actor|GetAllActorsOfClass "/Game/Test/BP_SecurityCamera.BP_SecurityCamera_C"))
  (bind _asbp_security_camera (Utilities|Casting|CastToBP_SecurityCamera (Utilities|Array|Get(acopy) _outactors)))
  (Variables|/Game/Test/BP_SecurityCamera.BP_SecurityCamera_C|SetCanShowCamera _asbp_security_camera true)
  (bind _returnvalue_2 (UserInterface|CreateWidget "/Game/Test/WBP_GameplayUI.WBP_GameplayUI_C"))
  (UserInterface|Viewport|AddtoViewport _returnvalue_2 0))

(event Input|KeyboardEvents|Escape
  (params (Key :type Key%20Structure :default "None"))
  (:Pressed
    (Utilities|FlowControl|FlipFlop
      (:A
        (Variables|Default|SetIsCursorVisible false))
      (:B
        (Variables|Default|SetIsCursorVisible true)))
    (Variables|/Script/Engine.PlayerController|SetbShowMouseCursor (Game|GetPlayerController 0) (Variables|Default|GetIsCursorVisible))))

(fn ConstructionScript)